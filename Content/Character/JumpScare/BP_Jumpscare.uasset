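; Jumpscare actor that fires when its Box is overlapped or when it is interacted with, and always reports as interactable.
; Both triggers call Scare through separate DoOnce gates, so each can fire it once.
; Scare unhides the mesh, blends the first player controller's view to this actor, loops a running animation and plays a 2D sound.
; The overlap has no actor filter, and the view is never restored here.
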(event `Scare`
  (`SceneComponent.SetHiddenInGame` (`self.Mesh`) false false)
  (`PlayerController.SetViewTargetWithBlend` (`GameplayStatics.GetPlayerController` 0) self 0.3 "VTBlend_Linear" 0.0 false)
  (`SkeletalMeshComponent.PlayAnimation` (`self.Mesh`) "/Game/Character/NPC/Enemy/student_1/animations/Fast_Run.Fast_Run" true)
  (`GameplayStatics.PlaySound2D` "/Game/Audio/Jumpscare.Jumpscare" 1.0 1.0 0.0 null null))

(event `/Game/Blueprint/InterFaces/BPI_Interact.OnInteract`
  (params (`Interacting Play` :type "Character Object Reference"))
  (`/Engine/EditorBlueprintResources/StandardMacros.DoOnce` false
    (:`Completed`
      (`self.Scare`))))

(event `self.Box.OnComponentBeginOverlap`
  (params (OverlappedComponent :type "PrimitiveComponent Object Reference") (OtherActor :type "Actor Object Reference") (OtherComp :type "PrimitiveComponent Object Reference") (OtherBodyIndex :type Integer) (bFromSweep :type Boolean) (SweepResult :type "HitResult Structure (by ref)"))
  (`/Engine/EditorBlueprintResources/StandardMacros.DoOnce` false
    (:`Completed`
      (`self.Scare`))))

(fn `IsInteractable`
  (returns (Interactable :type Boolean))
  (return true))

(fn `UserConstructionScript`)