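; BP_triggerJump is a one-shot trigger volume that fires a jump scare on the player's DL_Character.
; BeginPlay casts and caches player character 0.
; The first Box begin overlap calls JumpScare and the first end overlap calls JumpScaareOff, each gated by its own DoOnce with no reset.
; Neither overlap event checks which actor entered or left the box.
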(event `self.ReceiveBeginPlay`
  (bind _asdl_character (cast `/Game/Character/Player/DL_Character` (`GameplayStatics.GetPlayerCharacter` 0)))
  (set `self.Chara Ref` _asdl_character))

(event `self.Box.OnComponentBeginOverlap`
  (params (OverlappedComponent :type "PrimitiveComponent Object Reference") (OtherActor :type "Actor Object Reference") (OtherComp :type "PrimitiveComponent Object Reference") (OtherBodyIndex :type Integer) (bFromSweep :type Boolean) (SweepResult :type "HitResult Structure (by ref)"))
  (`/Engine/EditorBlueprintResources/StandardMacros.DoOnce` false
    (:`Completed`
      (`/Game/Character/Player/DL_Character.JumpScare` (`self.Chara Ref`)))))

(event `self.Box.OnComponentEndOverlap`
  (params (OverlappedComponent :type "PrimitiveComponent Object Reference") (OtherActor :type "Actor Object Reference") (OtherComp :type "PrimitiveComponent Object Reference") (OtherBodyIndex :type Integer))
  (`/Engine/EditorBlueprintResources/StandardMacros.DoOnce` false
    (:`Completed`
      (`/Game/Character/Player/DL_Character.JumpScaareOff` (`self.Chara Ref`)))))

(fn `UserConstructionScript`)