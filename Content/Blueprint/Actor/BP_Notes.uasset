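; BP_Notes is an interactable note actor that the player can read.
; On interact it copies its note description to the character reference, sets the Reading flag, plays a paper pickup sound, and calls ShowNote after a short delay.
; When an overlap with its box component ends, it hides the note and clears the Reading flag.
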(event `/Game/Blueprint/InterFaces/BPI_Interact.OnInteract`
  (params (`Interacting Play` :type "Character Object Reference"))
  (bind _chara_ref (`self.Chara Ref`))
  (set `/Game/Character/Player/DL_Character.Note` (`self.NoteDescription`) (`self.Chara Ref`))
  (set `/Game/Character/Player/DL_Character.Reading?` true _chara_ref)
  (`GameplayStatics.PlaySound2D` "/Game/Audio/paperpick.paperpick" 1.0 1.0 0.0 null null)
  (`KismetSystemLibrary.Delay` 0.2)
  (`/Game/Character/Player/DL_Character.ShowNote` _chara_ref))

(event `self.Box.OnComponentEndOverlap`
  (params (OverlappedComponent :type "PrimitiveComponent Object Reference") (OtherActor :type "Actor Object Reference") (OtherComp :type "PrimitiveComponent Object Reference") (OtherBodyIndex :type Integer))
  (`/Game/Character/Player/DL_Character.HideNote` (`self.Chara Ref`))
  (set `/Game/Character/Player/DL_Character.Reading?` false (`self.Chara Ref`)))

(fn `IsInteractable`
  (returns (Interactable :type Boolean))
  (return true))

(fn `UserConstructionScript`
  (`parent.UserConstructionScript`))