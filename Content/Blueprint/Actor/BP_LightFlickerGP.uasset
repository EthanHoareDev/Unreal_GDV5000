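; BP_LightFlickerGP is a light actor that flickers continuously during play.
; The construction script applies the normal Intensity to the Light component.
; From BeginPlay, a self-looping retriggerable delay waits a random time between Min and Max, then a FlipFlop alternates the light between MinIntensity and Intensity, producing irregular two-level flicker without Tick.
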(event `self.ReceiveBeginPlay`
  (bind _light (`self.Light`))
  (`KismetSystemLibrary.RetriggerableDelay` (`KismetMathLibrary.RandomFloatInRange` (`self.Min`) (`self.Max`)) :!label _label)
  (`/Engine/EditorBlueprintResources/StandardMacros.FlipFlop`
    (:`A`
      (`LightComponent.SetIntensity` _light (`self.MinIntensity`))
      (goto _label))
    (:`B`
      (`LightComponent.SetIntensity` _light (`self.Intensity`))
      (goto _label))))

(fn `UserConstructionScript`
  (`LightComponent.SetIntensity` (`self.Light`) (`self.Intensity`)))